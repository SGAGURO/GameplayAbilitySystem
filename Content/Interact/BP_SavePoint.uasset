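; BP_SavePoint is an interactable save point that writes the save game and lights up once used.
; Interact sets the EverActived flag, calls WriteSaveGame on the CGameMode, prints a green confirmation and runs the EverActived event.
; That event activates the particle system if the flag is set, and OnActorLoaded calls it too so the effect can return after loading.
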(event Custom|EverActived
  (if (Variables|Default|GetbEverActived)
    (Components|Activation|SetActive (Variables|Default|GetParticleSystem) true false)))

(event EventBeginPlay)

(event EventInteract
  (params (InstigatorPawn :type Pawn%20Object%20Reference))
  (Variables|Default|SetbEverActived true)
  (bind _ascgame_mode (Utilities|Casting|CastToCGameMode (Game|GetGameMode)))
  (Class|CGameMode|WriteSaveGame _ascgame_mode)
  (Development|PrintString "Saved by save point" true true "(R=0.172875,G=1.000000,B=0.259621,A=1.000000)")
  (CallFunction|EverActived))

(event EventOnActorLoaded
  (CallFunction|EverActived))

(fn ConstructionScript)