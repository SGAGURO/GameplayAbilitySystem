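; BP_Barrel is an explosive barrel that reacts to player interaction and to physical hits.
; Interact fires the RadialForce impulse and spawns a scaled-up explosion particle at the mesh location.
; A mesh hit from an actor with a CAttributeComponent reduces that actor's health and fires the same impulse, without the particle effect.
; The barrel is never destroyed, so both reactions can repeat.
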(event OnComponentHit(StaticMesh)
  (params (HitComponent :type Primitive%20Component%20Object%20Reference) (OtherActor :type Actor%20Object%20Reference) (OtherComp :type Primitive%20Component%20Object%20Reference) (NormalImpulse :type Vector :default "0, 0, 0") (Hit :type Hit%20Result%20Structure%20%28by%20ref%29))
  (bind _returnvalue (Actor|GetComponentbyClass OtherActor "/Script/GAS.CAttributeComponent"))
  (Utilities|IsValid OtherActor
    (:Is%20Valid
      (Utilities|IsValid _returnvalue
        (:Is%20Valid
          (Class|CAttributeComponent|ApplyHealthChange _returnvalue -3e+01)
          (Class|RadialForceComponent|FireImpulse (Variables|Default|GetRadialForce)))))))

(event EventInteract
  (params (InstigatorPawn :type Pawn%20Object%20Reference))
  (Class|RadialForceComponent|FireImpulse (Variables|Default|GetRadialForce))
  (Effects|SpawnEmitteratLocation "/Game/ExampleContent/Effects/P_Explosion.P_Explosion" (Transformation|GetWorldLocation (Variables|Default|GetStaticMesh)) "0, 0, 0" "5.000000,5.000000,5.000000"))

(fn ConstructionScript)