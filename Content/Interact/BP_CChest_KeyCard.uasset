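; A chest variant that opens only for a pawn holding the required key card.
; On Interact it checks the instigator's action component gameplay tags for the RequiredKey tag, then either runs the parent interaction or prints a colored missing-key message.
; The construction script applies the Emissive color to every static mesh component's materials, so the chest and its warning text share one color.
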(event EventInteract
  (params (InstigatorPawn :type Pawn%20Object%20Reference))
  (if (GameplayTags|HasTag (Variables|/Script/GAS.CActionComponent|GetActiveGameplayTags (Actor|GetComponentbyClass InstigatorPawn "/Script/GAS.CActionComponent")) (Variables|Chest|GetRequiredKey))
    (|CallParentFunction InstigatorPawn)
    (else
      (Development|PrintString (Utilities|String|Append (GameplayTags|GetDebugStringfromGameplayTag (Variables|Chest|GetRequiredKey)) " 키카드가 없다.") true true (Variables|Chest|GetEmissive)))))

(fn ConstructionScript
  (|CallParentFunction)
  (for _array_element (Actor|GetComponentsByClass "/Script/Engine.StaticMeshComponent")
    (Rendering|Material|SetVectorParameterValueonMaterials _array_element "Emissive" (Math|Conversions|ToVector(LinearColor) (Variables|Chest|GetEmissive)))))