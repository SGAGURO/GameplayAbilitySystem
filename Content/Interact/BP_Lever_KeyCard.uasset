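; BP_Lever_KeyCard is an interactable lever variant that grants key card access to the pawn that uses it.
; On Interact it runs the parent behavior, then adds the CardKey gameplay tag to the ActiveGameplayTags of the instigator's CActionComponent.
; The construction script calls its parent, then applies the Color variable to StaticMesh1's material Color parameter.
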(event EventInteract
  (params (InstigatorPawn :type Pawn%20Object%20Reference))
  (|CallParentFunction InstigatorPawn)
  (GameplayTags|AddGameplayTag (Variables|/Script/GAS.CActionComponent|GetActiveGameplayTags (Actor|GetComponentbyClass InstigatorPawn "/Script/GAS.CActionComponent")) (Variables|Default|GetCardKey) :!class /Script/GameplayTags.BlueprintGameplayTagLibrary))

(fn ConstructionScript
  (|CallParentFunction)
  (Rendering|Material|SetVectorParameterValueonMaterials (Variables|Default|GetStaticMesh1) "Color" (Math|Conversions|ToVector(LinearColor) (Variables|Default|GetColor))))